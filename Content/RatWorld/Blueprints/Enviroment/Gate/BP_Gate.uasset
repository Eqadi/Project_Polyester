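; BP_Gate is a gate that opens once every actor carrying its trigger tag is gone from the level.
; Tick polls two channels, GateOpen for Gate1 and GateOpen2 for Gate2, each firing once per gate instance.
; An empty channel makes that instance loop over all matching gates, flare their lights, jump animations to opening and destroy capsules.
; A delayed light removal follows inside the loop.
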(event `self.ReceiveActorBeginOverlap`
  (params (OtherActor :type "Actor Object Reference")))

(event `self.ReceiveTick`
  (params (DeltaSeconds :type "Float (single-precision)"))
  (`|ExecutionSequence`
    (:`then_0`
      (bind _outactors (`GameplayStatics.GetAllActorsWithTag` "GateOpen"))
      (if (< (+ (`KismetArrayLibrary.Array_Length` _outactors) 1) 2)
        (`/Engine/EditorBlueprintResources/StandardMacros.DoOnce` false
          (:`Completed`
            (bind _outactors_2 (`GameplayStatics.GetAllActorsOfClassWithTag` "BP_Gate_C" "Gate1"))
            (for _array_element _outactors_2
              (set `self.Gate` _array_element)
              (`|ExecutionSequence`
                (:`then_0`
                  (`LightComponent.SetIntensity` (`/Game/RatWorld/Blueprints/Enviroment/Gate/BP_Gate.PointLight` (`self.Gate`)) 100000.0))
                (:`then_1`
                  (`PaperZDAnimInstance.JumpToNode` (`self.GetAnimInstance` _array_element) "OpeningJump" "None")
                  (`ActorComponent.K2_DestroyComponent` (`/Game/RatWorld/Blueprints/Enviroment/Gate/BP_Gate.OnCapsule` (`self.Gate`)))
                  (`KismetSystemLibrary.Delay` 1.0)
                  (`ActorComponent.K2_DestroyComponent` (`/Game/RatWorld/Blueprints/Enviroment/Gate/BP_Gate.PointLight` (`self.Gate`))))))))))
    (:`then_1`
      (bind _outactors_3 (`GameplayStatics.GetAllActorsWithTag` "GateOpen2"))
      (if (< (+ (`KismetArrayLibrary.Array_Length` _outactors_3) 1) 2)
        (`/Engine/EditorBlueprintResources/StandardMacros.DoOnce` false
          (:`Completed`
            (bind _outactors_4 (`GameplayStatics.GetAllActorsOfClassWithTag` "BP_Gate_C" "Gate2"))
            (for _array_element_2 _outactors_4
              (set `self.Gate2` _array_element_2)
              (`|ExecutionSequence`
                (:`then_0`
                  (`LightComponent.SetIntensity` (`/Game/RatWorld/Blueprints/Enviroment/Gate/BP_Gate.PointLight` (`self.Gate2`)) 100000.0))
                (:`then_1`
                  (`PaperZDAnimInstance.JumpToNode` (`self.GetAnimInstance` _array_element_2) "OpeningJump" "None")
                  (`ActorComponent.K2_DestroyComponent` (`/Game/RatWorld/Blueprints/Enviroment/Gate/BP_Gate.OnCapsule` (`self.Gate2`)))
                  (`KismetSystemLibrary.Delay` 1.0)
                  (`ActorComponent.K2_DestroyComponent` (`/Game/RatWorld/Blueprints/Enviroment/Gate/BP_Gate.PointLight` (`self.Gate2`))))))))))))

(fn `UserConstructionScript`)
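; Game mode for a local two-player platform level that spawns, possesses and restarts BP_Boy_ZD characters.
; BeginPlay creates players at tagged PlayerStarts with per-player input mappings, binds defeat to RestartPlayer, plays music and adds lights to tagged rats and gates.
; Tick polls each player's RatTeleport tag; once none remain, that player teleports once to a fixed height with a one-second spotlight flash.
; A separate RestartGame function reloads the current level.
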(event `PlayerDefeat` :!signature `self.OnPlayerDefeat`
  (params (Boy :type "Character Object Reference"))
  (`self.RestartPlayer` (`Pawn.GetController` Boy)))

(event `self.ReceiveBeginPlay`
  (`|ExecutionSequence`
    (:`then_0`
      (`KismetSystemLibrary.Delay` 0.2)
      (`self.Create Players`))
    (:`then_1`
      (add `self.OnPlayerDefeat` (delegate `PlayerDefeat`)))
    (:`then_2`
      (`GameplayStatics.PlaySound2D` "/Game/RatWorld/Sounds/music.music" 1.0 1.0 0.0 null null))
    (:`then_3`
      (bind _outactors (`GameplayStatics.GetAllActorsOfClassWithTag` "/Game/RatWorld/Blueprints/Characters/Rat/BP_Rat_ZD.BP_Rat_ZD_C" "RatTeleport"))
      (for _array_element _outactors
        (`AddComponent|NODE_AddPointLightComponent-0` :`self` _array_element)))
    (:`then_4`
      (bind _outactors_2 (`GameplayStatics.GetAllActorsWithTag` "GateOpen"))
      (for _array_element_2 _outactors_2
        (`AddComponent|NODE_AddPointLightComponent-1` :`self` _array_element_2)))
    (:`then_5`
      (bind _outactors_3 (`GameplayStatics.GetAllActorsOfClassWithTag` "/Game/RatWorld/Blueprints/Characters/Rat/BP_Rat_ZD.BP_Rat_ZD_C" "RatTeleport2"))
      (for _array_element_3 _outactors_3
        (`AddComponent|NODE_AddPointLightComponent-2` :`self` _array_element_3)))
    (:`then_6`
      (bind _outactors_4 (`GameplayStatics.GetAllActorsWithTag` "GateOpen2"))
      (for _array_element_4 _outactors_4
        (`AddComponent|NODE_AddPointLightComponent-3` :`self` _array_element_4)))))

(event `self.ReceiveTick`
  (params (DeltaSeconds :type "Float (single-precision)"))
  (bind (_returnvalue_x _returnvalue_y) (`KismetMathLibrary.BreakVector` (`self.K2_GetActorLocation` (`self.As BP Boy ZD`))))
  (bind (_returnvalue_x_2 _returnvalue_y_2) (`KismetMathLibrary.BreakVector` (`self.K2_GetActorLocation` (`self.As BP Boy ZD2`))))
  (`|ExecutionSequence`
    (:`then_0`
      (bind _asbp_boy_zd (cast `/Game/RatWorld/Blueprints/Characters/Boy/BP_Boy_ZD` (`GameplayStatics.GetPlayerPawn` 0)))
      (set `self.As BP Boy ZD` _asbp_boy_zd)
      (bind _outactors (`GameplayStatics.GetAllActorsWithTag` "RatTeleport"))
      (if (and (not (`self.JumpTrigger`)) (< (+ (`KismetArrayLibrary.Array_Length` _outactors) 1) 2))
        (`/Engine/EditorBlueprintResources/StandardMacros.DoOnce` false
          (:`Completed`
            (`|ExecutionSequence`
              (:`then_0`
                (`LightComponent.SetIntensity` (`/Game/RatWorld/Blueprints/Characters/Boy/BP_Boy_ZD.SpotLight` (`self.As BP Boy ZD`)) 1500000.0))
              (:`then_1`
                (`self.K2_SetActorLocation` (`self.As BP Boy ZD`) (`KismetMathLibrary.MakeVector` _returnvalue_x _returnvalue_y -7100.0) false false)
                (`|ExecutionSequence`
                  (:`then_0`
                    (set `self.JumpTrigger` true))
                  (:`then_1`
                    (`KismetSystemLibrary.Delay` 1.0)
                    (`LightComponent.SetIntensity` (`/Game/RatWorld/Blueprints/Characters/Boy/BP_Boy_ZD.SpotLight` (`self.As BP Boy ZD`)) 0.0)))))))))
    (:`then_1`
      (bind _asbp_boy_zd_2 (cast `/Game/RatWorld/Blueprints/Characters/Boy/BP_Boy_ZD` (`GameplayStatics.GetPlayerPawn` 1)))
      (set `self.As BP Boy ZD2` _asbp_boy_zd_2)
      (bind _outactors_2 (`GameplayStatics.GetAllActorsWithTag` "RatTeleport2"))
      (if (and (not (`self.JumpTrigger2`)) (< (+ (`KismetArrayLibrary.Array_Length` _outactors_2) 1) 2))
        (`/Engine/EditorBlueprintResources/StandardMacros.DoOnce` false
          (:`Completed`
            (`|ExecutionSequence`
              (:`then_0`
                (`LightComponent.SetIntensity` (`/Game/RatWorld/Blueprints/Characters/Boy/BP_Boy_ZD.SpotLight` (`self.As BP Boy ZD2`)) 150000.0))
              (:`then_1`
                (`self.K2_SetActorLocation` (`self.As BP Boy ZD2`) (`KismetMathLibrary.MakeVector` _returnvalue_x_2 _returnvalue_y_2 -7100.0) false false)
                (`|ExecutionSequence`
                  (:`then_0`
                    (set `self.JumpTrigger2` true))
                  (:`then_1`
                    (`KismetSystemLibrary.Delay` 1.0)
                    (`LightComponent.SetIntensity` (`/Game/RatWorld/Blueprints/Characters/Boy/BP_Boy_ZD.SpotLight` (`self.As BP Boy ZD2`)) 0.0)))))))))))

(fn `Create Players`
  (bind _returnvalue (`GameplayStatics.GetPlayerController` (`self.Index`)))
  (bind _returnvalue_2 (pcsubsystem `EnhancedInputLocalPlayerSubsystem` (`GameplayStatics.GetPlayerController` (`self.Index`))))
  (bind _outactors (`GameplayStatics.GetAllActorsOfClass` "/Script/Engine.PlayerStart"))
  (for (_ _array_index) _outactors
    (bind _output_get (set `self.Index` _array_index))
    (if (== (`self.Index`) 0)
      (bind _outactors_2 (`GameplayStatics.GetAllActorsOfClassWithTag` "/Script/Engine.PlayerStart" "Start1"))
      (for _array_element _outactors_2
        (`GameplayStatics.CreatePlayer` _output_get)
        (`EnhancedInputSubsystemInterface.AddMappingContext` _returnvalue_2 "/Game/RatWorld/Input/Hero_ZD_Mapping.Hero_ZD_Mapping" 0 (struct))
        (bind _returnvalue_3 (`|SpawnActorFromClass` "/Game/RatWorld/Blueprints/Characters/Boy/BP_Boy_ZD.BP_Boy_ZD_C" (`self.GetTransform` _array_element) "Undefined" "MultiplyWithRoot" null null))
        (`Controller.Possess` _returnvalue _returnvalue_3))
      (else
        (bind _outactors_3 (`GameplayStatics.GetAllActorsOfClassWithTag` "/Script/Engine.PlayerStart" "Start2"))
        (for _array_element_2 _outactors_3
          (`GameplayStatics.CreatePlayer` _output_get)
          (`EnhancedInputSubsystemInterface.AddMappingContext` _returnvalue_2 "/Game/RatWorld/Input/Hero_ZD_Mapping2.Hero_ZD_Mapping2" 0 (struct))
          (bind _returnvalue_4 (`|SpawnActorFromClass` "/Game/RatWorld/Blueprints/Characters/Boy/BP_Boy_ZD.BP_Boy_ZD_C" (`self.GetTransform` _array_element_2) "Undefined" "MultiplyWithRoot" null null))
          (`Controller.Possess` _returnvalue _returnvalue_4))))))

(fn `RestartGame`
  (bind _returnvalue (`GameplayStatics.GetCurrentLevelName` true))
  (`GameplayStatics.OpenLevel` (`KismetStringLibrary.Conv_StringToName` _returnvalue)))

(fn `UserConstructionScript`)
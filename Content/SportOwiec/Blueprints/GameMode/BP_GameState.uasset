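; Game state for a two-player local ball match: creates the second player, spawns the ball and runs scoring to 10 points.
; After each point it respawns the ball by scorer and restarts both characters; a win clears points and starts over.
; Ball touch events count consecutive touches, awarding the opponent a foul point past the limit, with a flag blocking double scoring.
; Main menu creation is disconnected, so matches start immediately.
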(event `self.ReceiveBeginPlay`
  ;[1 1 1] Display main menu and Creating local player, characters are autopossesed
  (`self.StartMenu`)
  (`GameplayStatics.CreatePlayer` -1))

(event `StartMenu`
  (`self.DisableInput` (`GameplayStatics.GetPlayerCharacter` 0) (`GameplayStatics.GetPlayerController` 0))
  (`self.StartGame` :!label _label))

(event `OnStartGame_Event`
  (clear `/Game/SportOwiec/Blueprints/UI/WBP_MainMenu.OnStartGame` (`self.MainMenu`))
  ;[1 1 1] Comment
  (set `self.MainMenu` null)
  (goto _label))

(event `ShowWidget`
  (bind _returnvalue (`|CreateWidget` "/Game/SportOwiec/Blueprints/UI/BP_MainWidget.BP_MainWidget_C" (`GameplayStatics.GetPlayerController` 0)))
  (bind _output_get (set `self.MainWidget` _returnvalue))
  (`UserWidget.AddToViewport` _output_get 0))

(event `EndGame`
  (`self.K2_DestroyActor` (`self.MainBall`))
  (`Widget.RemoveFromParent` (`self.MainWidget`))
  (`self.StartMenu`)
  (`self.ClearPoints` (`GameplayStatics.GetPlayerState` 0))
  (`self.ClearPoints` (`GameplayStatics.GetPlayerState` 1)))

(event `StartGame`
  (`self.ShowWidget`)
  (`self.SpawnBall` (`KismetMathLibrary.RandomInteger` 2))
  (`self.EnableInput` (`GameplayStatics.GetPlayerCharacter` 0) (`GameplayStatics.GetPlayerController` 0))
  (`self.RestartCharactrer` (`GameplayStatics.GetPlayerCharacter` 1))
  (`self.RestartCharactrer` (`GameplayStatics.GetPlayerCharacter` 0)))

(event `ClearPoints`
  (params (PlayerState :type "PlayerState Object Reference"))
  (bind _asbp_player_state (cast `/Game/SportOwiec/Blueprints/GameMode/BP_PlayerState` PlayerState))
  (`/Game/SportOwiec/Blueprints/GameMode/BP_PlayerState.SetPoints` _asbp_player_state 0))

(event `AddPoints`
  (params (PlayerState :type "PlayerState Object Reference") (WasFoul :type Boolean))
  (if (`self.bPointCanBeAdded`)
    (set `self.bPointCanBeAdded` false)
    (`self.OnPointScored` PlayerState WasFoul)
    (bind _asbp_player_state (cast `/Game/SportOwiec/Blueprints/GameMode/BP_PlayerState` PlayerState))
    (`/Game/SportOwiec/Blueprints/GameMode/BP_PlayerState.AddPoints` _asbp_player_state 1)
    (set `self.Won` _asbp_player_state)
    (if (>= (`/Game/SportOwiec/Blueprints/GameMode/BP_PlayerState.GetPoints` _asbp_player_state) 10)
      (`KismetSystemLibrary.Delay` 1.0)
      (`self.EndGame`)
      (else
        (`KismetSystemLibrary.Delay` 1.0)
        (`self.RestartGame` (`self.Won`))))))

(event `RestartGame`
  (params (WhoWon :type "/Game/SportOwiec/Blueprints/GameMode/BP_PlayerState Object Reference"))
  (`self.K2_DestroyActor` (`self.MainBall`))
  (`self.SpawnBall` (`KismetMathLibrary.SelectInt` 0 1 (== WhoWon (`GameplayStatics.GetPlayerState` 0))))
  (`self.RestartCharactrer` (`GameplayStatics.GetPlayerCharacter` 1))
  (`self.RestartCharactrer` (`GameplayStatics.GetPlayerCharacter` 0)))

(event `SpawnBall`
  (params (Index :type Integer))
  (set `self.LastToucher` null)
  (`self.SetTouchCounter` 0)
  (bind _returnvalue (`|SpawnActorFromClass` "/Game/SportOwiec/Blueprints/Actors/BP_Ball.BP_Ball_C" (`KismetMathLibrary.MakeTransform` (`self.K2_GetActorLocation` (`BlueprintMapLibrary.Map_Find` (`self.SpawnPoints`) Index))) "Undefined" "MultiplyWithRoot" self null))
  (bind _output_get (set `self.MainBall` _returnvalue))
  (`self.OnBallSpawned` _output_get)
  (add `/Game/SportOwiec/Blueprints/Actors/BP_Ball.OnPlayerTouch` (`self.MainBall`) (delegate `OnPlayerTouch_Event`))
  (set `self.bPointCanBeAdded` true))

(event `RestartCharactrer`
  (params (Character :type "Character Object Reference"))
  (bind _asbp_player_character (cast `/Game/SportOwiec/Blueprints/Characters/BP_PlayerCharacter` Character))
  (`/Game/SportOwiec/Blueprints/Characters/BP_PlayerCharacter.Restart` _asbp_player_character))

(event `OnPlayerTouch_Event`
  (params (Character :type "/Game/SportOwiec/Blueprints/Characters/BP_PlayerCharacter Object Reference"))
  (`self.BallPlayerTouch` Character))

(event `BallPlayerTouch`
  (params (Character :type "/Game/SportOwiec/Blueprints/Characters/BP_PlayerCharacter Object Reference"))
  (`|ExecutionSequence`
    (:`then_0`
      (if (== Character (`self.LastToucher`))
        (`self.AddTouchCounter` 1)
        (if (`self.bPointCanBeAdded`)
          (if (>= (`self.GetTouchCounter`) 3)
            (`|ExecutionSequence`
              (:`then_0`
                (bind _asplayer_controller (cast `PlayerController` (`Pawn.GetController` (`self.LastToucher`))))
                (`self.AddPoints` (`GameplayStatics.GetPlayerState` (select `int` (`GameplayStatics.GetPlayerControllerID` _asplayer_controller) :`0` 1 :`1` 0)) true))
              (:`then_1`
                (set `self.bPointCanBeAdded` false)))))
        (else
          (`self.SetTouchCounter` 0))))
    (:`then_1`
      (set `self.LastToucher` Character))))

(fn `AddRegisterSpawnPoint`
  (params (Key :type "Integer (by ref)") (Value :type "/Game/SportOwiec/Blueprints/Actors/BP_SpawnBallLocation Object Reference (by ref)"))
  (`BlueprintMapLibrary.Map_Add` (`self.SpawnPoints`) Key Value))

(fn `AddTouchCounter`
  (params (Touch :type Integer))
  (`self.SetTouchCounter` (+ Touch (`self.GetTouchCounter`))))

(fn `GetTouchCounter`
  (returns (TouchCounter :type Integer))
  (return (`self.TouchCounter`)))

(fn `SetTouchCounter`
  (params (TouchCounter :type Integer))
  (bind _output_get (set `self.TouchCounter` TouchCounter))
  (`self.OnTouchCounter` _output_get))

(fn `UserConstructionScript`)
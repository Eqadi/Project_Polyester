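; BP_Ball is a physical game ball that players knock around, using projectile movement locked to the YZ plane by resetting its starting X every tick.
; Player hits report a debounced touch and, on a first hit or fast player, enable gravity and launch the ball away from the impact at fixed speed.
; Every hit spawns a flash effect, while a throttled, pitch-varied bounce sound plays on the first or sufficiently fast hits.
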(event `self.Sphere1.OnComponentHit`
  (params (HitComponent :type "PrimitiveComponent Object Reference") (OtherActor :type "Actor Object Reference") (OtherComp :type "PrimitiveComponent Object Reference") (NormalImpulse :type "Vector Structure") (Hit :type "HitResult Structure (by ref)"))
  (bind (_bblockinghit _binitialoverlap _time _distance _location _impactpoint) (`GameplayStatics.BreakHitResult` Hit))
  (bind _returnvalue (`self.GetVelocity`))
  (`|ExecutionSequence`
    (:`then_0`
      (bind _asbp_player_character (cast `/Game/Sportowiec/Blueprints/Characters/BP_PlayerCharacter` OtherActor))
      (`|ExecutionSequence`
        (:`then_0`
          (if (> (- (`GameplayStatics.GetTimeSeconds`) (`self.LastTouch`)) 0.1)
            (set `self.LastTouch` (`GameplayStatics.GetTimeSeconds`))
            (`self.OnPlayerTouch` _asbp_player_character)))
        (:`then_1`
          (if (or (> (`KismetMathLibrary.VSize` (`self.GetVelocity` _asbp_player_character)) 100.0) (`self.FirstHit`))
            (set `ProjectileMovementComponent.ProjectileGravityScale` 1.0 (`self.ProjectileMovement`))
            (set `MovementComponent.Velocity` (* (`KismetMathLibrary.Vector_NormalUnsafe` (* (- (`SceneComponent.K2_GetComponentLocation` (`self.Sphere1`)) _impactpoint) (0.0 1.0 1.0))) 1000.0) (`self.ProjectileMovement`))))))
    (:`then_1`
      (`NiagaraFunctionLibrary.SpawnSystemAtLocation` "/Game/VFX/Niagara/ToonProjectiles2/Effects/NS_Flash_11.NS_Flash_11" _impactpoint)
      (if (or (`self.FirstHit`) (and (> (`KismetMathLibrary.VSize` _returnvalue) 60.0) (> (`KismetMathLibrary.Abs` (.z _returnvalue)) 50.0)))
        (set `self.FirstHit` false)
        (if (> (- (`GameplayStatics.GetTimeSeconds`) (`self.LastSound`)) 0.4)
          (set `self.LastSound` (`GameplayStatics.GetTimeSeconds`))
          (`GameplayStatics.SpawnSoundAtLocation` "/Game/Sportowiec/Audio/WAV_Bounce.WAV_Bounce" (`self.K2_GetActorLocation`) (struct) 55.0 (`KismetMathLibrary.RandomFloatInRange` 0.9 1.1) 0.0 "/Game/Sportowiec/Audio/SA_Attenuation.SA_Attenuation" null))))))

(event `self.Sphere2.OnComponentBeginOverlap`
  (params (OverlappedComponent :type "PrimitiveComponent Object Reference") (OtherActor :type "Actor Object Reference") (OtherComp :type "PrimitiveComponent Object Reference") (OtherBodyIndex :type Integer) (bFromSweep :type Boolean) (SweepResult :type "HitResult Structure (by ref)")))

(event `self.ReceiveTick`
  (params (DeltaSeconds :type "Float (single-precision)"))
  (bind _newvar_x (`KismetMathLibrary.BreakVector` (`self.NewVar`)))
  (`self.K2_SetActorLocation` (`KismetMathLibrary.MakeVector_NetQuantize` _newvar_x (.y (`self.K2_GetActorLocation`)) (.z (`self.K2_GetActorLocation`)))))

(event `self.ReceiveBeginPlay`
  (set `self.NewVar` (`self.K2_GetActorLocation`)))

(fn `UserConstructionScript`)
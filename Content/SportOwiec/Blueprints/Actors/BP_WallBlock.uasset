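; BP_WallBlock is a scoring wall that awards points through BP_GameState when a BP_Ball overlaps its box.
; By default the point goes to the player at PlayerIndexOwner.
; With CheckForFoul on, a ball last touched by that player's character is a foul, so the point goes to the other player of the two, flagged as a foul.
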(event `self.Box.OnComponentBeginOverlap`
  (params (OverlappedComponent :type "PrimitiveComponent Object Reference") (OtherActor :type "Actor Object Reference") (OtherComp :type "PrimitiveComponent Object Reference") (OtherBodyIndex :type Integer) (bFromSweep :type Boolean) (SweepResult :type "HitResult Structure (by ref)"))
  (cast `/Game/Sportowiec/Blueprints/Actors/BP_Ball` OtherActor)
  (if (`self.CheckForFoul`)
    (bind _returnvalue (`self.IsFoul`))
    (if _returnvalue
      (`self.AddPointstoPlayerByIndex` (select `int` (`self.PlayerIndexOwner`) :`0` 1 :`1` 0) true)
      (else
        (`self.AddPointstoPlayerByIndex` (`self.PlayerIndexOwner`) :!label _label)))
    (else
      (goto _label))))

(event `AddPointstoPlayerByIndex`
  (params (PlayerStateIndex :type Integer) (WasFoul :type Boolean))
  (bind _asbp_game_state (cast `/Game/Sportowiec/Blueprints/GameMode/BP_GameState` (`GameplayStatics.GetGameState`)))
  (`/Game/Sportowiec/Blueprints/GameMode/BP_GameState.AddPoints` _asbp_game_state (`GameplayStatics.GetPlayerState` PlayerStateIndex) WasFoul))

(fn `IsFoul`
  (returns (ReturnValue :type Boolean))
  (bind _asbp_game_state (cast `/Game/Sportowiec/Blueprints/GameMode/BP_GameState` (`GameplayStatics.GetGameState`)))
  (return (== (`/Game/Sportowiec/Blueprints/GameMode/BP_GameState.LastToucher` _asbp_game_state) (`GameplayStatics.GetPlayerCharacter` (`self.PlayerIndexOwner`)))))

(fn `UserConstructionScript`)
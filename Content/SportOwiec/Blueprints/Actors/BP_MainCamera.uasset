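; Main camera actor that tracks the ball spawned by the game state, with a constant breathing camera shake.
; Each tick it shifts along X and Z with the ball's height, keeping Y fixed and never dropping below its spawn position.
; The camera rotates toward an interpolated look-at point that follows the ball.
; Marker components in the actor, mostly arrows, bound the camera's height and the look-at point's Y/Z range.
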(event `self.ReceiveBeginPlay`
  (set `self.SpawnLocation` (`self.K2_GetActorLocation`))
  (`PlayerCameraManager.StartCameraShake` :`self` (`PlayerController.PlayerCameraManager` (`GameplayStatics.GetPlayerController` 0)) :`ShakeClass` "/Game/Sportowiec/CameraShake/CS_Breath.CS_Breath_C")
  (bind _asbp_game_state (cast `/Game/Sportowiec/Blueprints/GameMode/BP_GameState` (`GameplayStatics.GetGameState`)))
  (add `/Game/Sportowiec/Blueprints/GameMode/BP_GameState.OnBallSpawned` _asbp_game_state (delegate `OnBallSpawned_Event`)))

(event `OnBallSpawned_Event`
  (params (Ball :type "Actor Object Reference"))
  (bind _output_get (set `self.Ball` Ball))
  (set `self.LookAt` (`self.K2_GetActorLocation` _output_get)))

(event `self.ReceiveTick`
  (params (DeltaSeconds :type "Float (single-precision)"))
  (bind (_returnvalue_x _returnvalue_y) (`KismetMathLibrary.BreakVector` (`SceneComponent.K2_GetComponentLocation` (`self.Arrow`))))
  (bind (_returnvalue_x_2 _returnvalue_y_2) (`KismetMathLibrary.BreakVector` (`SceneComponent.K2_GetComponentLocation` (`self.Arrow1`))))
  (bind (_returnvalue_x_3 _returnvalue_y_3 _returnvalue_z) (`KismetMathLibrary.BreakVector` (`SceneComponent.K2_GetComponentLocation` (`self.Arrow2`))))
  (bind (_returnvalue_x_4 _returnvalue_y_4 _returnvalue_z_2) (`KismetMathLibrary.BreakVector` (`SceneComponent.K2_GetComponentLocation` (`self.MaxBallLookAt`))))
  (bind _ball (`self.Ball`)
    (:`then`
      (bind _returnvalue (`self.K2_GetActorLocation` _ball))
      (bind _z (.z _returnvalue))
      (`self.K2_SetActorLocation` (`KismetMathLibrary.MakeVector` (`KismetMathLibrary.FClamp` (.x (+ (`self.SpawnLocation`) (`KismetMathLibrary.MakeVector` (* (- _z 300.0) 0.3)))) (.x (`self.SpawnLocation`)) 9999999.0) (.y (`self.SpawnLocation`)) (`KismetMathLibrary.FClamp` (/ _z 3.0) (.z (`self.SpawnLocation`)) _returnvalue_z)))
      (bind _output_get (set `self.LookAt` (`KismetMathLibrary.MakeVector` (.x (`KismetMathLibrary.VInterpTo` (`self.LookAt`) _returnvalue DeltaSeconds 4.0)) (`KismetMathLibrary.FClamp` (.y (`KismetMathLibrary.VInterpTo` (`self.LookAt`) _returnvalue DeltaSeconds 4.0)) _returnvalue_y _returnvalue_y_2) (`KismetMathLibrary.FClamp` (.z (`KismetMathLibrary.VInterpTo` (`self.LookAt`) _returnvalue DeltaSeconds 4.0)) 0.0 _returnvalue_z_2))))
      (`SceneComponent.K2_SetWorldRotation` (`self.Camera`) (`KismetMathLibrary.FindLookAtRotation` (`self.K2_GetActorLocation`) _output_get) false false))
    (:`else`)))

(fn `UserConstructionScript`)
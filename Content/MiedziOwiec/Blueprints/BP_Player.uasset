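; Player pawn acting as a gold-miner style hook that swings back and forth, fires along its angle and reels in loot for points.
; Tick oscillates the pitch until Player 1 input locks a direction, then pushes the pawn forward with movement input.
; Overlapping gold, bag, diamond or rock attaches it and tweens back over a time scaled by distance and PullUpSpeed, then destroys it.
; Player 2 input is unimplemented.
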(event `self.ReceiveBeginPlay`
  (`KismetSystemLibrary.Delay` 0.2)
  (set `self.HookStartLocation` (`self.K2_GetActorLocation`))
  (bind _asbp_player_controller (cast `/Game/MiedziOwiec/Blueprints/BP_PlayerController` (`self.GetController`)))
  (`EnhancedInputSubsystemInterface.AddMappingContext` (pcsubsystem `EnhancedInputLocalPlayerSubsystem` _asbp_player_controller) "/Game/MiedziOwiec/Blueprints/IMC_Miedz_1.IMC_Miedz_1" 0 (struct)))

(event `EnhancedInput|/Game/MiedziOwiec/Blueprints/IA_Movement_Player1`
  (params (ActionValue :type "Float (double-precision)") (ElapsedSeconds :type "Float (double-precision)") (TriggeredSeconds :type "Float (double-precision)") (InputAction :type "InputAction Object Reference" :default "/Game/MiedziOwiec/Blueprints/IA_Movement_Player1.IA_Movement_Player1"))
  (:`Triggered`
    (`self.HookDown`)))

(event `EnhancedInput|/Game/MiedziOwiec/Blueprints/IA_Movement_Player2`
  (params (ActionValue :type "Float (double-precision)") (ElapsedSeconds :type "Float (double-precision)") (TriggeredSeconds :type "Float (double-precision)") (InputAction :type "InputAction Object Reference" :default "/Game/MiedziOwiec/Blueprints/IA_Movement_Player2.IA_Movement_Player2")))

(event `self.ReceiveActorBeginOverlap`
  (params (OtherActor :type "Actor Object Reference")))

(event `HookDown`
  (bind _pitch (.pitch (`self.K2_GetActorRotation`)))
  (bind _result (`/Engine/EditorBlueprintResources/StandardMacros.NegateFloat` (`KismetMathLibrary.Abs` (`KismetMathLibrary.DegCos` _pitch)))
    (:`  `
      (set `self.HookDirectionVector` (`KismetMathLibrary.MakeVector` (`KismetMathLibrary.DegSin` _pitch) 0.0 _result))
      (set `self.Rotating` false)
      (set `self.MoveHookForward` true))))

(event `self.ReceiveTick`
  (params (DeltaSeconds :type "Float (single-precision)"))
  (bind _yrotation (`self.YRotation`))
  (if (`self.Rotating`)
    (`KismetSystemLibrary.Delay` 0.02)
    (`self.K2_SetActorRotation` (`KismetMathLibrary.MakeRotator` 0.0 (`self.YRotation`)) true)
    (if (`self.Adding`)
      (`/Engine/EditorBlueprintResources/StandardMacros.CompareFloat` _yrotation 65.0
        (:`==`
          (set `self.Adding` false))
        (:`<`
          (set `self.YRotation` (+ _yrotation 1.0))))
      (else
        (`/Engine/EditorBlueprintResources/StandardMacros.CompareFloat` _yrotation -65.0
          (:`>`
            (set `self.YRotation` (- _yrotation 1.0)))
          (:`==`
            (set `self.Adding` true)))))
    (elif (`self.MoveHookForward`)
      (`self.AddMovementInput` (`self.HookDirectionVector`)))))

(event `self.CapsuleComponent.OnComponentBeginOverlap`
  (params (OverlappedComponent :type "PrimitiveComponent Object Reference") (OtherActor :type "Actor Object Reference") (OtherComp :type "PrimitiveComponent Object Reference") (OtherBodyIndex :type Integer) (bFromSweep :type Boolean) (SweepResult :type "HitResult Structure (by ref)"))
  (bind _asbp_gold (cast `/Game/MiedziOwiec/Blueprints/BP_Gold` OtherActor)
    (:`then`
      (`self.MoveBackHook` _asbp_gold (`/Game/MiedziOwiec/Blueprints/BP_Gold.PullUpSpeed` _asbp_gold) (`/Game/MiedziOwiec/Blueprints/BP_Gold.PointsValue` _asbp_gold)))
    (:`CastFailed`
      (bind _asbp_bag (cast `/Game/MiedziOwiec/Blueprints/BP_Bag` OtherActor)
        (:`then`
          (`self.MoveBackHook` _asbp_bag (`/Game/MiedziOwiec/Blueprints/BP_Bag.PullUpSpeed` _asbp_bag) (`/Game/MiedziOwiec/Blueprints/BP_Bag.PointsValue` _asbp_bag)))
        (:`CastFailed`
          (bind _asbp_diamond (cast `/Game/MiedziOwiec/Blueprints/BP_Diamond` OtherActor)
            (:`then`
              (`self.MoveBackHook` _asbp_diamond (`/Game/MiedziOwiec/Blueprints/BP_Diamond.PullUpSpeed` _asbp_diamond) (`/Game/MiedziOwiec/Blueprints/BP_Diamond.PointsValue` _asbp_diamond)))
            (:`CastFailed`
              (bind _asbp_rock (cast `/Game/MiedziOwiec/Blueprints/BP_Rock` OtherActor))
              (`self.MoveBackHook` _asbp_rock (`/Game/MiedziOwiec/Blueprints/BP_Rock.PullUpSpeed` _asbp_rock) (`/Game/MiedziOwiec/Blueprints/BP_Rock.PointsValue` _asbp_rock)))))))))

(event `MoveBackHook`
  (params (CaughtObject :type "Object Object Reference") (PullUpSpeed :type "Float (double-precision)") (PointsValue :type Integer))
  (bind _returnvalue (`self.K2_GetActorLocation` self))
  (bind _returnvalue_2 (`self.K2_GetActorRotation` self))
  (bind _hookstartlocation (`self.HookStartLocation`))
  (bind _rootcomponent (`self.RootComponent`))
  (set `self.MoveHookForward` false)
  (bind _asactor (cast `Actor` CaughtObject)
    (:`then`
      (`self.K2_AttachToActor` _asactor self "None" "SnapToTarget" "SnapToTarget" "SnapToTarget" true)
      (bind _timetopullup (`self.CalculateTimeToPullUp` PullUpSpeed _hookstartlocation _returnvalue))
      (`KismetSystemLibrary.MoveComponentTo` _rootcomponent _hookstartlocation _returnvalue_2 false false _timetopullup)
      (set `self.Rotating` true)
      (`self.K2_DestroyActor` _asactor)
      (set `self.Points` (+ PointsValue (`self.Points`))))
    (:`CastFailed`
      (bind _timetopullup_2 (`self.CalculateTimeToPullUp` PullUpSpeed _hookstartlocation _returnvalue))
      (`KismetSystemLibrary.MoveComponentTo` _rootcomponent _hookstartlocation _returnvalue_2 false false _timetopullup_2)
      (set `self.Rotating` true))))

(fn `CalculateTimeToPullUp`
  (params (PullUpSpeed :type "Float (double-precision)") (StartLocation :type "Vector Structure") (EndLocation :type "Vector Structure"))
  (returns (TimeToPullUp :type "Float (double-precision)"))
  (return (* PullUpSpeed (/ (`KismetMathLibrary.Vector_Distance` StartLocation EndLocation) 100.0))))

(fn `UserConstructionScript`)
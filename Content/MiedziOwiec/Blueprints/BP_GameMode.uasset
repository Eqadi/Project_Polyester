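; Game mode that sets up local multiplayer by creating and spawning a player for each PlayerStart in the level.
; Shortly after BeginPlay it loops over the starts, creating a controller per index and possessing a new pawn: BP_Player for the first, BP_Player1 for the rest.
; A parallel sequence branch opens the level named by LevelName after a fixed 15-second delay.
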(event `self.ReceiveBeginPlay`
  (bind _returnvalue (`GameplayStatics.GetPlayerController` (`self.arrayindex`)))
  (`|ExecutionSequence`
    (:`then_0`
      (`KismetSystemLibrary.Delay` 0.2)
      (bind _outactors (`GameplayStatics.GetAllActorsOfClass` "/Script/Engine.PlayerStart"))
      (for (_array_element _array_index) _outactors
        (bind _output_get (set `self.arrayindex` _array_index))
        (if (== (`self.arrayindex`) 0)
          (`GameplayStatics.CreatePlayer` _output_get)
          (bind _returnvalue_2 (`self.GetTransform` _array_element))
          (bind _returnvalue_3 (`|SpawnActorFromClass` "/Game/MiedziOwiec/Blueprints/BP_Player.BP_Player_C" _returnvalue_2 "Undefined" "MultiplyWithRoot" null null))
          (`Controller.Possess` _returnvalue _returnvalue_3)
          (else
            (`GameplayStatics.CreatePlayer` _output_get)
            (bind _returnvalue_4 (`|SpawnActorFromClass` "/Game/MiedziOwiec/Blueprints/BP_Player1.BP_Player1_C" _returnvalue_2 "Undefined" "MultiplyWithRoot" null null))
            (`Controller.Possess` _returnvalue _returnvalue_4)))))
    (:`then_1`
      (`KismetSystemLibrary.Delay` 15.0)
      (`GameplayStatics.OpenLevel` (`self.Level Name`)))))

(fn `UserConstructionScript`)
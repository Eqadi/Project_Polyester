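; Bars actor that clears its Box and NSSpeedFlowerV2 components once either of two players has BarsEnter2 set.
; While Temp is true, Tick casts player 0 to BP_ThirdPersonCharacter, then player 1 to BP_ThirdPersonCharacter2 if needed, to poll that flag.
; When it is set, both components are destroyed and Temp turns false; when neither player has it, both stay visible.
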(event `self.ReceiveTick`
  (params (DeltaSeconds :type "Float (single-precision)"))
  (if (`self.Temp`)
    (bind _asbp_third_person_character (cast `/Game/ThirdPerson/Blueprints/BP_ThirdPersonCharacter` (`GameplayStatics.GetPlayerCharacter` 0)))
    (if (`/Game/ThirdPerson/Blueprints/BP_ThirdPersonCharacter.Bars_enter_2` _asbp_third_person_character)
      (`ActorComponent.K2_DestroyComponent` (`self.Box`) :!label _label)
      (`ActorComponent.K2_DestroyComponent` (`self.NS_Speed_Flower_v2`))
      (set `self.Temp` false)
      (else
        (bind _asbp_third_person_character_2 (cast `/Game/ThirdPerson/Blueprints/BP_ThirdPersonCharacter2` (`GameplayStatics.GetPlayerCharacter` 1)))
        (if (`/Game/ThirdPerson/Blueprints/BP_ThirdPersonCharacter2.Bars_enter_2` _asbp_third_person_character_2)
          (goto _label)
          (else
            (`SceneComponent.SetVisibility` (`self.NS_Speed_Flower_v2`) true false)
            (`SceneComponent.SetVisibility` (`self.Box`) true false)))))))

(fn `UserConstructionScript`)
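; BP_Open_portal is a portal trigger that reacts separately to the two player character Blueprints through two capsules.
; Capsule responds to BP_ThirdPersonCharacter and Capsule1 to BP_ThirdPersonCharacter2, setting that character's PortalEnter flag on overlap and clearing it on exit.
; Entry also plays a sound at world origin and hides the whole actor through its root.
; Either exit shows it again, regardless of the other capsule.
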(event `self.Capsule.OnComponentBeginOverlap`
  (params (OverlappedComponent :type "PrimitiveComponent Object Reference") (OtherActor :type "Actor Object Reference") (OtherComp :type "PrimitiveComponent Object Reference") (OtherBodyIndex :type Integer) (bFromSweep :type Boolean) (SweepResult :type "HitResult Structure (by ref)"))
  (bind _asbp_third_person_character (cast `/Game/ThirdPerson/Blueprints/BP_ThirdPersonCharacter` OtherActor))
  (if true
    (`GameplayStatics.PlaySoundAtLocation` "/Game/Assets3D/Audio/ooo1.ooo1" (0.0 0.0 0.0) (struct) 1.0 1.0 0.0 null null null null)
    (set `/Game/ThirdPerson/Blueprints/BP_ThirdPersonCharacter.portal_enter` true _asbp_third_person_character)
    (`SceneComponent.SetVisibility` (`self.DefaultSceneRoot`) false true :!label _label)))

(event `self.Capsule1.OnComponentBeginOverlap`
  (params (OverlappedComponent :type "PrimitiveComponent Object Reference") (OtherActor :type "Actor Object Reference") (OtherComp :type "PrimitiveComponent Object Reference") (OtherBodyIndex :type Integer) (bFromSweep :type Boolean) (SweepResult :type "HitResult Structure (by ref)"))
  (bind _asbp_third_person_character_2 (cast `/Game/ThirdPerson/Blueprints/BP_ThirdPersonCharacter2` OtherActor))
  (`GameplayStatics.PlaySoundAtLocation` "/Game/Assets3D/Audio/ooo2.ooo2" (0.0 0.0 0.0) (struct) 1.0 1.0 0.0 null null null null)
  (set `/Game/ThirdPerson/Blueprints/BP_ThirdPersonCharacter2.portal_enter` true _asbp_third_person_character_2)
  (goto _label))

(event `self.Capsule.OnComponentEndOverlap`
  (params (OverlappedComponent :type "PrimitiveComponent Object Reference") (OtherActor :type "Actor Object Reference") (OtherComp :type "PrimitiveComponent Object Reference") (OtherBodyIndex :type Integer))
  (bind _asbp_third_person_character (cast `/Game/ThirdPerson/Blueprints/BP_ThirdPersonCharacter` OtherActor))
  (set `/Game/ThirdPerson/Blueprints/BP_ThirdPersonCharacter.portal_enter` false _asbp_third_person_character)
  (`SceneComponent.SetVisibility` (`self.DefaultSceneRoot`) true true :!label _label_2))

(event `self.Capsule1.OnComponentEndOverlap`
  (params (OverlappedComponent :type "PrimitiveComponent Object Reference") (OtherActor :type "Actor Object Reference") (OtherComp :type "PrimitiveComponent Object Reference") (OtherBodyIndex :type Integer))
  (bind _asbp_third_person_character_2 (cast `/Game/ThirdPerson/Blueprints/BP_ThirdPersonCharacter2` OtherActor))
  (set `/Game/ThirdPerson/Blueprints/BP_ThirdPersonCharacter2.portal_enter` false _asbp_third_person_character_2)
  (goto _label_2))

(fn `UserConstructionScript`)
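; BP_Mak_Collect_gold is a gold collectible that awards 10 Mak points to whichever of two player character types picks it up.
; Two overlap capsules each accept one character class, BP_ThirdPersonCharacter or BP_ThirdPersonCharacter2, adding to that character's own points variable and playing its own sound.
; On pickup it hides the whole actor and disables collision on both capsules instead of destroying itself, so it can only be collected once.
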(event `self.Capsule1.OnComponentBeginOverlap`
  (params (OverlappedComponent :type "PrimitiveComponent Object Reference") (OtherActor :type "Actor Object Reference") (OtherComp :type "PrimitiveComponent Object Reference") (OtherBodyIndex :type Integer) (bFromSweep :type Boolean) (SweepResult :type "HitResult Structure (by ref)"))
  (bind _asbp_third_person_character (cast `/Game/ThirdPerson/Blueprints/BP_ThirdPersonCharacter` OtherActor))
  (`GameplayStatics.PlaySoundAtLocation` "/Game/Assets3D/Audio/maaak1.maaak1" (0.0 0.0 0.0) (struct) 1.0 1.0 0.0 null null null null)
  (set `/Game/ThirdPerson/Blueprints/BP_ThirdPersonCharacter.Mak_points_1` (+ (`/Game/ThirdPerson/Blueprints/BP_ThirdPersonCharacter.Mak_points_1` _asbp_third_person_character) 10) _asbp_third_person_character)
  (`SceneComponent.SetVisibility` (`self.DefaultSceneRoot`) false true)
  (`PrimitiveComponent.SetCollisionEnabled` (`self.Capsule2`) "NoCollision")
  (`PrimitiveComponent.SetCollisionEnabled` (`self.Capsule1`) "NoCollision"))

(event `self.Capsule2.OnComponentBeginOverlap`
  (params (OverlappedComponent :type "PrimitiveComponent Object Reference") (OtherActor :type "Actor Object Reference") (OtherComp :type "PrimitiveComponent Object Reference") (OtherBodyIndex :type Integer) (bFromSweep :type Boolean) (SweepResult :type "HitResult Structure (by ref)"))
  (bind _asbp_third_person_character_2 (cast `/Game/ThirdPerson/Blueprints/BP_ThirdPersonCharacter2` OtherActor))
  (`GameplayStatics.PlaySoundAtLocation` "/Game/Assets3D/Audio/Maaak2.Maaak2" (0.0 0.0 0.0) (struct) 1.0 1.0 0.0 null null null null)
  (set `/Game/ThirdPerson/Blueprints/BP_ThirdPersonCharacter2.Mak_points_2` (+ (`/Game/ThirdPerson/Blueprints/BP_ThirdPersonCharacter2.Mak_points_2` _asbp_third_person_character_2) 10) _asbp_third_person_character_2)
  (`SceneComponent.SetVisibility` (`self.DefaultSceneRoot`) false true)
  (`PrimitiveComponent.SetCollisionEnabled` (`self.Capsule2`) "NoCollision")
  (`PrimitiveComponent.SetCollisionEnabled` (`self.Capsule1`) "NoCollision"))

(fn `UserConstructionScript`)
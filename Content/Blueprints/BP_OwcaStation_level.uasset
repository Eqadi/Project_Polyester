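; Level exit station for two characters that opens the level named by LevelName once both are in place and E is pressed.
; Box and Box1 overlaps flag one character class each, and E registers only while the first flag is set.
; Both begin-overlap events poll these flags through Delay loops before opening the level.
; Each end-overlap clears the other box's flag, not its own, plus the E confirmation.
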(event `self.ReceiveBeginPlay`
  (`self.EnableInput` (`GameplayStatics.GetPlayerController` 0)))

(event `Key|E`
  (params (Key :type "Key Structure"))
  (:`Pressed`
    (if (`self.Enter_1`)
      (set `self.Enter_11` true)
      (if true
        _))))

(event `self.Box.OnComponentBeginOverlap`
  (params (OverlappedComponent :type "PrimitiveComponent Object Reference") (OtherActor :type "Actor Object Reference") (OtherComp :type "PrimitiveComponent Object Reference") (OtherBodyIndex :type Integer) (bFromSweep :type Boolean) (SweepResult :type "HitResult Structure (by ref)"))
  (cast `/Game/ThirdPerson/Blueprints/BP_ThirdPersonCharacter` OtherActor)
  (set `self.Enter_1` true)
  (if (`self.Enter_1`) :!label _label
    (if (`self.Enter_11`)
      (if (`self.Enter_2`)
        (if true :!label _label_2
          (`GameplayStatics.OpenLevel` (`self.Level Name`)))
        (else
          (`KismetSystemLibrary.Delay` 0.1 :!label _label_3)
          (goto _label)))
      (else
        (goto _label_3)))))

(event `self.Box1.OnComponentBeginOverlap`
  (params (OverlappedComponent :type "PrimitiveComponent Object Reference") (OtherActor :type "Actor Object Reference") (OtherComp :type "PrimitiveComponent Object Reference") (OtherBodyIndex :type Integer) (bFromSweep :type Boolean) (SweepResult :type "HitResult Structure (by ref)"))
  (cast `/Game/ThirdPerson/Blueprints/BP_ThirdPersonCharacter2` OtherActor)
  (set `self.Enter_2` true)
  (if (`self.Enter_1`) :!label _label_4
    (if (`self.Enter_11`)
      (goto _label_2)
      (else
        (`KismetSystemLibrary.Delay` 0.5)
        (goto _label_4)))))

(event `self.Box.OnComponentEndOverlap`
  (params (OverlappedComponent :type "PrimitiveComponent Object Reference") (OtherActor :type "Actor Object Reference") (OtherComp :type "PrimitiveComponent Object Reference") (OtherBodyIndex :type Integer))
  (cast `/Game/ThirdPerson/Blueprints/BP_ThirdPersonCharacter` OtherActor)
  (set `self.Enter_2` false)
  (set `self.Enter_11` false))

(event `self.Box1.OnComponentEndOverlap`
  (params (OverlappedComponent :type "PrimitiveComponent Object Reference") (OtherActor :type "Actor Object Reference") (OtherComp :type "PrimitiveComponent Object Reference") (OtherBodyIndex :type Integer))
  (cast `/Game/ThirdPerson/Blueprints/BP_ThirdPersonCharacter2` OtherActor)
  (set `self.Enter_1` false)
  (set `self.Enter_11` false))

(fn `UserConstructionScript`)
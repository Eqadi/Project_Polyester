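; BP_Water_MinusPoints is a water hazard that drains points from the two third-person characters while they are in it.
; Separate trigger boxes track each character type: Box for BP_ThirdPersonCharacter, Box1 for BP_ThirdPersonCharacter2.
; Each overlap starts a Delay loop that decrements that character's points immediately, then every second until its InWater flag clears on exit.
; Only the first character's loop stops at zero; the second has no zero check.
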(event `self.ReceiveBeginPlay`)

(event `self.Box.OnComponentBeginOverlap`
  (params (OverlappedComponent :type "PrimitiveComponent Object Reference") (OtherActor :type "Actor Object Reference") (OtherComp :type "PrimitiveComponent Object Reference") (OtherBodyIndex :type Integer) (bFromSweep :type Boolean) (SweepResult :type "HitResult Structure (by ref)"))
  (bind _inwater1 (`self.InWater1`))
  (bind _asbp_third_person_character (cast `/Game/ThirdPerson/Blueprints/BP_ThirdPersonCharacter` OtherActor))
  (set `self.InWater1` true)
  (bind _mak_points_1 (`/Game/ThirdPerson/Blueprints/BP_ThirdPersonCharacter.Mak_points_1` _asbp_third_person_character))
  (if (not (== _mak_points_1 0)) :!label _label
    (`/Engine/EditorBlueprintResources/StandardMacros.DecrementInt` _mak_points_1
      (:`  `
        (if _inwater1
          (`KismetSystemLibrary.Delay` 1.0)
          (if _inwater1
            (goto _label)))))))

(event `self.Box.OnComponentEndOverlap`
  (params (OverlappedComponent :type "PrimitiveComponent Object Reference") (OtherActor :type "Actor Object Reference") (OtherComp :type "PrimitiveComponent Object Reference") (OtherBodyIndex :type Integer))
  (cast `/Game/ThirdPerson/Blueprints/BP_ThirdPersonCharacter` OtherActor)
  (set `self.InWater1` false))

(event `self.Box1.OnComponentBeginOverlap`
  (params (OverlappedComponent :type "PrimitiveComponent Object Reference") (OtherActor :type "Actor Object Reference") (OtherComp :type "PrimitiveComponent Object Reference") (OtherBodyIndex :type Integer) (bFromSweep :type Boolean) (SweepResult :type "HitResult Structure (by ref)"))
  (bind _inwater2 (`self.inWater2`))
  (bind _asbp_third_person_character_2 (cast `/Game/ThirdPerson/Blueprints/BP_ThirdPersonCharacter2` OtherActor))
  (set `self.inWater2` true)
  (`/Engine/EditorBlueprintResources/StandardMacros.DecrementInt` (`/Game/ThirdPerson/Blueprints/BP_ThirdPersonCharacter2.Mak_points_2` _asbp_third_person_character_2) :!label _label_2
    (:`  `
      (if _inwater2
        (`KismetSystemLibrary.Delay` 1.0)
        (if _inwater2
          (goto _label_2))))))

(event `self.Box1.OnComponentEndOverlap`
  (params (OverlappedComponent :type "PrimitiveComponent Object Reference") (OtherActor :type "Actor Object Reference") (OtherComp :type "PrimitiveComponent Object Reference") (OtherBodyIndex :type Integer))
  (cast `/Game/ThirdPerson/Blueprints/BP_ThirdPersonCharacter2` OtherActor)
  (set `self.inWater2` false))

(fn `UserConstructionScript`)